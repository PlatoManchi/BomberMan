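; BP_RemoteBomb is a remote bomb actor with an animated cylinder and sound feedback.
; BeginPlay plays a press sound, and Explode calls the parent's explosion logic before playing a 2D explosion sound.
; Tick bobs the cylinder once per second by feeding the sine of an accumulating angle into a position lerp, whose negative alpha overshoots past the start point.
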(event `self.ReceiveBeginPlay`
  (`GameplayStatics.PlaySound2D` "/Game/Sounds/BOS_PRESS.BOS_PRESS"))

(event `self.ReceiveTick`
  (params (DeltaSeconds :type "Float (single-precision)"))
  ;[1 1 1] Move the remove up and down
  (bind _output_get (set `self.Angle` (+ (* DeltaSeconds 360.0) (`self.Angle`))))
  (`SceneComponent.K2_SetRelativeLocation` (`self.Cylinder`) (`KismetMathLibrary.VLerp` (0.0 -7.0 40.0) (0.0 0.0 27.0) (`KismetMathLibrary.DegSin` _output_get)) false false))

(event `self.Explode`
  (`parent.Explode`)
  (`GameplayStatics.PlaySound2D` "/Game/Sounds/Explosion.Explosion"))

(fn `UserConstructionScript`)